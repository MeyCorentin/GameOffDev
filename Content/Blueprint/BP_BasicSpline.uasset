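; BP_BasicSpline moves a referenced Follow actor along its spline at a speed set by SplineSpeed.
; Each Tick makes the actor's root Movable, re-attaches it to the spline and advances Distance by speed times delta time.
; It applies the spline's local location and rotation at that distance as a relative transform, preserving the actor's scale.
; Distance accumulates without wrapping or clamping to the spline length.
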(event `self.ReceiveTick`
  (params (DeltaSeconds :type "Float (single-precision)"))
  (bind (_returnvalue_location _returnvalue_rotation) (`KismetMathLibrary.BreakTransform` (`SplineComponent.GetTransformAtDistanceAlongSpline` (`self.Spline`) (`self.Distance`) "Local" false)))
  (`SceneComponent.SetMobility` (`Actor.RootComponent` (`self.Follow`)) "Movable")
  (`self.K2_AttachToComponent` (`self.Follow`) (`self.Spline`) "None" "KeepRelative" "KeepRelative" "KeepRelative" true)
  (set `self.Distance` (+ (* DeltaSeconds (`self.SplineSpeed`)) (`self.Distance`)))
  (`SceneComponent.K2_SetRelativeTransform` (`Actor.RootComponent` (`self.Follow`)) (`KismetMathLibrary.MakeTransform` _returnvalue_location _returnvalue_rotation (`self.GetActorRelativeScale3D` (`self.Follow`))) false false))

(fn `UserConstructionScript`)